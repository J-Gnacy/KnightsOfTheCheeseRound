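; Enemy character that attacks the player's BP_SirCheese, takes damage and adds one to the player's Score when destroyed.
; Hit flags whether the other actor is SirCheese and writes that to the AI Blackboard's "In range" key.
; Attack plays an animation and immediately damages SirCheese if in range, while Damaged destroys the enemy below 1 HP.
; Disconnected leftovers include projectile damage and behavior tree startup, which never run.
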(event Custom|Damaged
  (params (DamageAmount :type Integer))
  (Variables|Default|SetHP (- (Variables|Default|GetHP) DamageAmount))
  (if (< (Variables|Default|GetHP) 1)
    (Actor|DestroyActor)))

(event EventAttack
  (bind _attackanimation (Variables|Default|GetAttackAnimation))
  (Components|Animation|PlayAnimation (Variables|Character|GetMesh) _attackanimation false)
  (Animation|GetPlayLength _attackanimation)
  (if (Variables|Default|GetIn%20range)
    (bind _asbp_sir_cheese (Utilities|Casting|CastToBP_SirCheese (Variables|Default|GetComponentHit)))
    (Class|AdroidGamePawn|GetDamaged _asbp_sir_cheese)))

(event Collision|EventHit
  (params (MyComp :type Primitive%20Component%20Object%20Reference) (Other :type Actor%20Object%20Reference) (OtherComp :type Primitive%20Component%20Object%20Reference) (bSelfMoved :type Boolean) (HitLocation :type Vector :default "0, 0, 0") (HitNormal :type Vector :default "0, 0, 0") (NormalImpulse :type Vector :default "0, 0, 0") (Hit :type Hit%20Result%20Structure%20%28by%20ref%29))
  (bind _asbp_sir_cheese (Utilities|Casting|CastToBP_SirCheese Other)
    (:then
      (Variables|Default|SetComponentHit _asbp_sir_cheese)
      (Variables|Default|SetIn%20range true))
    (:CastFailed
      (Variables|Default|SetIn%20range false)))
  (AI|Components|Blackboard|SetValueasBool (Variables|/Script/AIModule.AIController|GetBlackboard (AI|GetAIController self)) (Utilities|Name|MakeLiteralName "In range") (Variables|Default|GetIn%20range)))

(event EventDestroyed
  (bind _asbp_sir_cheese (Utilities|Casting|CastToBP_SirCheese (Game|Player|GetPlayerPawn 0)))
  (Variables|/Script/AdroidGame.AdroidGamePawn|Setscore _asbp_sir_cheese (+ (Variables|/Script/AdroidGame.AdroidGamePawn|Getscore _asbp_sir_cheese) 1)))

(fn ConstructionScript)