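; BP_EnemySpawner is an actor that spawns a finite series of BP_Enemy actors at an accelerating pace, starting on BeginPlay.
; A custom Delayed For macro acts as a latent for loop, running its body and then waiting before the next index.
; Each iteration spawns an enemy and divides the Interval variable feeding that delay, so the gaps between spawns shrink geometrically.
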(event EventBeginPlay
  (|CallParentFunction)
  (Variables|Default|SetInterval 1e+01)
  (Utilities|Delayedfor 0 50 (Variables|Default|GetInterval)
    (:Loop%20Body
      (CallFunction|SpawnActor "/Game/Blueprints/Characters/BP_Enemy.BP_Enemy_C")
      (Variables|Default|SetInterval (/ (Variables|Default|GetInterval) 1.2)))))

(event Collision|EventActorBeginOverlap
  (params (OtherActor :type Actor%20Object%20Reference))
  (|CallParentFunction OtherActor) ; This node is disabled and will not be called.\nDrag off pins to build functionality.
)

(event EventTick
  (params (DeltaSeconds :type Float%20%28single-precision%29))
  (|CallParentFunction DeltaSeconds) ; This node is disabled and will not be called.\nDrag off pins to build functionality.
)

(fn ConstructionScript
  (|CallParentFunction))